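; Breakout ball for a Vive VR game that destroys bricks on impact.
; Any hit puts it in play, after which Tick enforces a minimum speed and subtracts gravity along X to pull it toward the player.
; Brick hits spawn an explosion and remove the brick from the Vive_Pawn's BrickWall.
; SetBallDynamics sets speed and gravity; the manual wall-bounce velocity reversal is disconnected.
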(event `Reverse X Velocity`
  (bind (_returnvalue_x _returnvalue_y _returnvalue_z) (`KismetMathLibrary.BreakVector` (`KismetMathLibrary.Normal` (`self.current_velocity`))))
  ;[0.4431 1 0.9302] Reverse X while maintaining constant velocity
  (set `self.new_velocity` (* (`KismetMathLibrary.MakeVector` (* _returnvalue_x -1.0) _returnvalue_y _returnvalue_z) 0.0)))

(event `Reverse Y Velocity`
  (bind (_returnvalue_x _returnvalue_y _returnvalue_z) (`KismetMathLibrary.BreakVector` (`KismetMathLibrary.Normal` (`self.current_velocity`))))
  (bind (_returnvalue_x_2 _returnvalue_y_2 _returnvalue_z_2) (`KismetMathLibrary.BreakVector` (* (`KismetMathLibrary.MakeVector` _returnvalue_x (* _returnvalue_y -1.0) _returnvalue_z) 0.0)))
  ;[0.4431 1 0.9302] Reverse Y while maintaining constant velocity
  (set `self.new_velocity` (`KismetMathLibrary.MakeVector` (- _returnvalue_x_2 (`self.gravity`)) _returnvalue_y_2 _returnvalue_z_2)))

(event `Reverse Z Velocity`
  (bind (_returnvalue_x _returnvalue_y _returnvalue_z) (`KismetMathLibrary.BreakVector` (`KismetMathLibrary.Normal` (`self.current_velocity`))))
  (bind (_returnvalue_x_2 _returnvalue_y_2 _returnvalue_z_2) (`KismetMathLibrary.BreakVector` (* (`KismetMathLibrary.MakeVector` _returnvalue_x _returnvalue_y (* _returnvalue_z -1.0)) 0.0)))
  ;[0.4431 1 0.9302] Reverse Z while maintaining constant velocity
  (set `self.new_velocity` (`KismetMathLibrary.MakeVector` (- _returnvalue_x_2 (`self.gravity`)) _returnvalue_y_2 _returnvalue_z_2)))

(event `self.ReceiveBeginPlay`
  ;[1 1 1] Create reference to Vive_Pawn to establish game and level state
  (bind _asvive_pawn (cast `/Game/Breakout/Player/Vive_Pawn` (`Controller.K2_GetPawn` (`GameplayStatics.GetPlayerController` 0)))
    (:`then`
      (set `self.VivePlayerPawn` _asvive_pawn))
    (:`CastFailed`
      (`KismetSystemLibrary.PrintString` "BALL FAILED TO GET VIVE_PAWN"))))

(event `self.ReceiveTick`
  (params (DeltaSeconds :type "Float (single-precision)"))
  (bind (_current_velocity_x _current_velocity_y _current_velocity_z) (`KismetMathLibrary.BreakVector` (`self.current_velocity`)))
  (bind (_returnvalue_x _returnvalue_y _returnvalue_z) (`KismetMathLibrary.BreakVector` (* (`KismetMathLibrary.Normal` (`self.current_velocity`)) (`self.minimum_speed`))))
  ;[1 1 1] find current position and velocity
  (if (`self.in_play`)
    (bind _returnvalue (`PrimitiveComponent.GetPhysicsLinearVelocity` (`self.Ball`) "None"))
    (set `self.current_velocity` _returnvalue)
    (set `self.current_pos` (`SceneComponent.K2_GetComponentLocation` (`self.Ball`)))
    (if (< (`KismetMathLibrary.VSize` (`self.current_velocity`)) (`self.minimum_speed`))
      (`PrimitiveComponent.SetPhysicsLinearVelocity` (`self.Ball`) (`KismetMathLibrary.MakeVector` (- _returnvalue_x (`self.gravity`)) _returnvalue_y _returnvalue_z) false "None") ; Ball is stucking going side to side, add gravity towards player
      (else
        (`PrimitiveComponent.SetPhysicsLinearVelocity` (`self.Ball`) (`KismetMathLibrary.MakeVector` (- _current_velocity_x (`self.gravity`)) _current_velocity_y _current_velocity_z) false "None")))))

(event `self.ReceiveHit`
  (params (MyComp :type "PrimitiveComponent Object Reference") (Other :type "Actor Object Reference") (OtherComp :type "PrimitiveComponent Object Reference") (bSelfMoved :type Boolean) (HitLocation :type "Vector Structure") (HitNormal :type "Vector Structure") (NormalImpulse :type "Vector Structure") (Hit :type "HitResult Structure (by ref)"))
  (set `self.in_play` true) ; Mark this ball as in play
  ;[1 1 1] Destroy bricks when hit
  (bind _asbrick (cast `/Game/Breakout/Blueprints/Brick` Other))
  (`|ExecutionSequence`
    (:`then_0`
      (bind (_returnvalue_x _returnvalue_y _returnvalue_z) (`KismetMathLibrary.BreakVector` (`self.K2_GetActorLocation` _asbrick)))
      (`GameplayStatics.SpawnEmitterAtLocation` "/Game/Breakout/ParticleSystems/ExplodingBricks/P_ExplodingBricks.P_ExplodingBricks" (`KismetMathLibrary.MakeVector` _returnvalue_x _returnvalue_y (+ _returnvalue_z 15.0))))
    (:`then_1`
      (`self.K2_DestroyActor` _asbrick)
      (`KismetArrayLibrary.Array_RemoveItem` (`/Game/Breakout/Player/Vive_Pawn.BrickWall` (`self.VivePlayerPawn`)) _asbrick))))

(fn `SetBallDynamics`
  (params (new_min_speed :type "Float (double-precision)") (new_gravity :type "Float (double-precision)"))
  (set `self.minimum_speed` new_min_speed)
  (set `self.gravity` new_gravity))

(fn `UserConstructionScript`
  (bind _returnvalue (`KismetMaterialLibrary.CreateDynamicMaterialInstance` "/Game/Breakout/Assets/Materials/M_Ball_Emissive_Inst.M_Ball_Emissive_Inst"))
  (bind _output_get (set `self.ball_brightness` _returnvalue))
  (`MaterialInstanceDynamic.SetScalarParameterValue` _output_get "brightness" 0.0)
  (`PrimitiveComponent.SetMaterial` (`self.Ball`) 0 _output_get))