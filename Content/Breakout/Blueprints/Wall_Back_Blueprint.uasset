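; Back wall fence for the Breakout game that flashes when the ball crosses it.
; The construction script puts a dynamic material instance on the mesh with fence brightness at zero.
; Any actor overlap, with no filter for the ball, restarts a timeline that drives that brightness parameter.
; On BeginPlay it also stores the mesh's world X as the back wall surface location.
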(event `self.ReceiveBeginPlay`
  (set `self.back_wall_surface_location` (.x (`SceneComponent.K2_GetComponentLocation` (`self.StaticMeshComponent`)))))

(event `self.ReceiveActorBeginOverlap`
  (params (OtherActor :type "Actor Object Reference"))
  ;[1 0.4208 0.9257] Flash fence when ball crosses
  (bind (_direction _emissive) (`Timeline|flash fence` :!via `PlayFromStart`)
    (:`Update`
      (`MaterialInstanceDynamic.SetScalarParameterValue` (`self.red_emissive`) "fence_brightness" _emissive))))

(fn `UserConstructionScript`
  (bind _returnvalue (`KismetMaterialLibrary.CreateDynamicMaterialInstance` "/Game/Materials/Fence_triggered_Inst.Fence_triggered_Inst"))
  (bind _output_get (set `self.red_emissive` _returnvalue))
  (`MaterialInstanceDynamic.SetScalarParameterValue` _output_get "fence_brightness" 0.0)
  (`PrimitiveComponent.SetMaterial` (`self.StaticMeshComponent`) 0 _output_get))