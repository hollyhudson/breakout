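; Ball actor for a VR brick-breaker that bounces inside a box and destroys any Brick it hits.
; BeginPlay takes side-wall limits from Vive_Pawn and hardcodes ceiling, floor and front limits.
; Tick compares position to those limits, flipping the matching velocity axis or otherwise drifting the ball along -X toward the player.
; The Hit handler's velocity tweak is never applied, as Tick overwrites CurrentVelocity from physics.
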(event `self.ReceiveBeginPlay`
  ;[1 1 1] get right and left wall boundaries
  (bind _outactors (`GameplayStatics.GetAllActorsOfClass` "/Game/Player/Vive_Pawn.Vive_Pawn_C"))
  (for _array_element _outactors
    (set `self.boundary_wall_l` (- (`/Game/Player/Vive_Pawn.left_wall_location` _array_element) 5.0))
    (set `self.boundary_wall_r` (+ (`/Game/Player/Vive_Pawn.right_wall_location` _array_element) 5.0))
    (set `self.boundary_ceiling` 281.0)
    (set `self.boundary_floor` 0.0)
    (set `self.boundary_wall_front` 814.0)
    (set `self.gravity` 2.0)))

(event `Reverse X Velocity`
  ;[1 1 1] Comment
  (set `self.new_velocity` (`KismetMathLibrary.MakeVector` (* (.x (`self.current_velocity`)) -1.0) (.y (`self.current_velocity`)) (.z (`self.current_velocity`)))))

(event `self.ReceiveTick`
  (params (DeltaSeconds :type "Float (single-precision)"))
  (bind (_current_velocity_x _current_velocity_y _current_velocity_z) (`KismetMathLibrary.BreakVector` (`self.current_velocity`)))
  ;[1 1 1] find current position and velocity
  (bind _returnvalue (`PrimitiveComponent.GetPhysicsLinearVelocity` (`self.Ball`) "None"))
  (set `self.current_velocity` _returnvalue)
  (bind _output_get (set `self.current_pos` (`SceneComponent.K2_GetComponentLocation` (`self.Ball`))))
  (bind _y (.y _output_get))
  (bind _z (.z _output_get))
  (if (> (.x _output_get) (`self.boundary_wall_front`))
    (`self.Reverse X Velocity`)
    (`PrimitiveComponent.SetPhysicsLinearVelocity` (`self.Ball`) (`self.new_velocity`) false "None" :!label _label)
    (elif (> _y (`self.boundary_wall_r`))
      (`self.Reverse Y Velocity` :!label _label_2)
      (goto _label)
      (elif (< _y (`self.boundary_wall_l`))
        (goto _label_2)
        (elif (> _z (`self.boundary_ceiling`))
          (`self.Reverse Z Velocity` :!label _label_3)
          (goto _label)
          (elif (< _z (`self.boundary_floor`))
            (goto _label_3)
            (else
              (`PrimitiveComponent.SetPhysicsLinearVelocity` (`self.Ball`) (`KismetMathLibrary.MakeVector` (- _current_velocity_x 2.0) _current_velocity_y _current_velocity_z) false "None") ; There has been no collision, enforce gravity towards player
            )))))))

(event `Reverse Y Velocity`
  ;[1 1 1] Comment
  (set `self.new_velocity` (`KismetMathLibrary.MakeVector` (- (.x (`self.current_velocity`)) (`self.gravity`)) (* (.y (`self.current_velocity`)) -1.0) (.z (`self.current_velocity`)))))

(event `Reverse Z Velocity`
  ;[1 1 1] Comment
  (set `self.new_velocity` (`KismetMathLibrary.MakeVector` (- (.x (`self.current_velocity`)) (`self.gravity`)) (.y (`self.current_velocity`)) (* (.z (`self.current_velocity`)) -1.0))))

(event `self.ReceiveHit`
  (params (MyComp :type "PrimitiveComponent Object Reference") (Other :type "Actor Object Reference") (OtherComp :type "PrimitiveComponent Object Reference") (bSelfMoved :type Boolean) (HitLocation :type "Vector Structure") (HitNormal :type "Vector Structure") (NormalImpulse :type "Vector Structure") (Hit :type "HitResult Structure (by ref)"))
  (if (`KismetMathLibrary.ClassIsChildOf` (`GameplayStatics.GetObjectClass` Other) "/Game/Blueprints/Brick.Brick_C")
    (`self.K2_DestroyActor` Other)
    (set `self.current_velocity` (`KismetMathLibrary.MakeVector` (+ (.x (`self.current_velocity`)) (`self.gravity`)) (.y (`self.current_velocity`)) (.z (`self.current_velocity`))))))

(fn `UserConstructionScript`)